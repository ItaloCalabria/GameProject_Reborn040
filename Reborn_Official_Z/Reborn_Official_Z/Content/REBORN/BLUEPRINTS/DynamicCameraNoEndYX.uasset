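; Trigger-volume camera actor that takes over the player's view when Edward_BluePrint enters StartCamera; leaving does not switch the view back.
; A self-recalling 0.005-second delay loop runs while the player is inside and this is the view target.
; If IsStationary, the camera rotates toward the player; otherwise the spring arm moves with the player on TrackPlayer-masked axes, taking others from actor location minus a first-entry offset.
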(event `self.StartCamera.OnComponentBeginOverlap`
  (params (OverlappedComponent :type "PrimitiveComponent Object Reference") (OtherActor :type "Actor Object Reference") (OtherComp :type "PrimitiveComponent Object Reference") (OtherBodyIndex :type Integer) (bFromSweep :type Boolean) (SweepResult :type "HitResult Structure (by ref)"))
  (cast `/Game/REBORN/BLUEPRINTS/Edward_BluePrint` OtherActor)
  (`PlayerController.SetViewTargetWithBlend` (`GameplayStatics.GetPlayerController` 0) self 0.0 "VTBlend_Linear" 0.0 false)
  (set `self.IsIn` true)
  (`self.CustomEvent_0`)
  (`/Engine/EditorBlueprintResources/StandardMacros.DoOnce` false
    (:`Completed`
      (set `self.Offset` (- (`self.K2_GetActorLocation` (`GameplayStatics.GetPlayerCharacter` 0)) (`SceneComponent.K2_GetComponentLocation` (`self.SpringArm`)))))))

(event `self.StartCamera.OnComponentEndOverlap`
  (params (OverlappedComponent :type "PrimitiveComponent Object Reference") (OtherActor :type "Actor Object Reference") (OtherComp :type "PrimitiveComponent Object Reference") (OtherBodyIndex :type Integer))
  (cast `/Game/REBORN/BLUEPRINTS/Edward_BluePrint` OtherActor)
  (set `self.IsIn` false)
  (`KismetSystemLibrary.PrintString` "cabouse"))

(event `CustomEvent_0`
  (`KismetSystemLibrary.Delay` 0.005)
  (if (== (`Controller.GetViewTarget` (`GameplayStatics.GetPlayerController` 0)) self)
    (if (`self.IsStationary`)
      (bind _rotation (`self.TrackPlayerRotation` 0.0))
      (`SceneComponent.K2_SetWorldRotation` (`self.Camera`) _rotation false false)
      (else
        (bind _vector (`self.TrackPlayerMovement` 0.0))
        (`SceneComponent.K2_SetWorldLocation` (`self.SpringArm`) _vector false false)))
    (`KismetSystemLibrary.PrintString` "Hello")
    (if (`self.IsIn`)
      (`self.CustomEvent_0`))))

(fn `TrackPlayerMovement`
  (params (`Delta Time` :type "Float (double-precision)"))
  (returns (Vector :type "Vector Structure"))
  (bind _trackplayer (`self.TrackPlayer`))
  (bind _returnvalue (- (`self.K2_GetActorLocation`) (`self.Offset`)))
  (return (`KismetMathLibrary.VInterpTo` _returnvalue (+ (* (`self.K2_GetActorLocation` (`GameplayStatics.GetPlayerCharacter` 0)) _trackplayer) (* _returnvalue (- (1.0 1.0 1.0) _trackplayer))) `Delta Time`)))

(fn `TrackPlayerRotation`
  (params (Delta :type "Float (double-precision)"))
  (returns (Rotation :type "Rotator Structure"))
  (return (`KismetMathLibrary.FindLookAtRotation` (`SceneComponent.K2_GetComponentLocation` (`self.Camera`)) (`self.K2_GetActorLocation` (`GameplayStatics.GetPlayerCharacter` 0)))))

(fn `UserConstructionScript`)