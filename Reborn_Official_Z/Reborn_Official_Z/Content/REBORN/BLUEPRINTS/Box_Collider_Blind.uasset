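; Interaction trigger that lets Edward enable throwing, apparently by taking an item from a toolbox, judging by the sound.
; Overlapping Trigger2 opens a gate for the Action input, which only proceeds while AllowThrow is false.
; A timeline turns Edward's yaw toward the actor, then calls SHOCKOFF and CanThrow, plays the sound and briefly disables input.
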(event `self.ReceiveBeginPlay`
  (bind _asedward_blue_print (cast `/Game/REBORN/BLUEPRINTS/Edward_BluePrint` (`GameplayStatics.GetPlayerCharacter` 0)))
  (set `self.Edward` _asedward_blue_print))

(event `InputAction|Action` :consume false
  (params (Key :type "Key Structure"))
  (bind _edward (`self.Edward`))
  (bind _edward_2 (`self.Edward`))
  (bind (_returnvalue_roll _returnvalue_pitch _returnvalue_yaw) (`KismetMathLibrary.BreakRotator` (`KismetMathLibrary.FindLookAtRotation` (`self.K2_GetActorLocation` _edward_2) (`self.K2_GetActorLocation`))))
  (:`Pressed`
    (`/Engine/EditorBlueprintResources/StandardMacros.Gate` true :!label _label
      (:`Exit`
        (if (not (`/Game/REBORN/BLUEPRINTS/Edward_BluePrint.Allow_Throw` _edward_2))
          (set `self.Rotation` (`self.K2_GetActorRotation` _edward_2))
          (bind (_direction _newtrack_0) (`Timeline|Timeline_0` :!via `PlayFromStart`)
            (:`Update`
              (`self.K2_SetActorRotation` _edward_2 (`KismetMathLibrary.RLerp` (`self.Rotation`) (`KismetMathLibrary.MakeRotator` 0.0 0.0 _returnvalue_yaw) _newtrack_0 true) false))
            (:`Finished`
              (`self.DisableInput` _edward null)
              (`/Game/REBORN/BLUEPRINTS/Edward_BluePrint.SHOCK_OFF` _edward)
              (`/Game/REBORN/BLUEPRINTS/Edward_BluePrint.CanThrow` _edward)
              (`GameplayStatics.PlaySound2D` "/Game/REBORN/SOUNDS/TAKE_FROM_TOOLBOX.TAKE_FROM_TOOLBOX" 1.0 1.0 0.0 null null)
              (`KismetSystemLibrary.Delay` 0.5)
              (`self.EnableInput` _edward null))))))))

(event `self.Trigger2.OnComponentBeginOverlap`
  (params (OverlappedComponent :type "PrimitiveComponent Object Reference") (OtherActor :type "Actor Object Reference") (OtherComp :type "PrimitiveComponent Object Reference") (OtherBodyIndex :type Integer) (bFromSweep :type Boolean) (SweepResult :type "HitResult Structure (by ref)"))
  (goto _label :!via `Open`))

(event `self.Trigger2.OnComponentEndOverlap`
  (params (OverlappedComponent :type "PrimitiveComponent Object Reference") (OtherActor :type "Actor Object Reference") (OtherComp :type "PrimitiveComponent Object Reference") (OtherBodyIndex :type Integer))
  (goto _label :!via `Close`))

(fn `UserConstructionScript`)