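; Box collider actor that turns the Edward player character to face it when the Action input is pressed inside its trigger.
; Trigger2 overlaps open and close a Gate on the input, without filtering which actor overlaps.
; A timeline lerps Edward from his current rotation to a yaw-only look-at rotation toward the collider.
; A DoOnce blocks repeat presses until the turn finishes.
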(event `self.ReceiveBeginPlay`
  (bind _asedward_blue_print (cast `/Game/REBORN/BLUEPRINTS/Edward_BluePrint` (`GameplayStatics.GetPlayerCharacter` 0)))
  (set `self.Edward` _asedward_blue_print))

(event `InputAction|Action` :consume false
  (params (Key :type "Key Structure"))
  (bind _edward (`self.Edward`))
  (bind (_returnvalue_roll _returnvalue_pitch _returnvalue_yaw) (`KismetMathLibrary.BreakRotator` (`KismetMathLibrary.FindLookAtRotation` (`self.K2_GetActorLocation` _edward) (`self.K2_GetActorLocation`))))
  (:`Pressed`
    (`/Engine/EditorBlueprintResources/StandardMacros.Gate` true :!label _label
      (:`Exit`
        (`/Engine/EditorBlueprintResources/StandardMacros.DoOnce` false :!label _label_2
          (:`Completed`
            (set `self.Rotation` (`self.K2_GetActorRotation` _edward))
            (bind (_direction _newtrack_0) (`Timeline|Timeline_0` :!via `PlayFromStart`)
              (:`Update`
                (`self.K2_SetActorRotation` _edward (`KismetMathLibrary.RLerp` (`self.Rotation`) (`KismetMathLibrary.MakeRotator` 0.0 0.0 _returnvalue_yaw) _newtrack_0) false))
              (:`Finished`
                (goto _label_2 :!via `Reset`)))))))))

(event `self.Trigger2.OnComponentBeginOverlap`
  (params (OverlappedComponent :type "PrimitiveComponent Object Reference") (OtherActor :type "Actor Object Reference") (OtherComp :type "PrimitiveComponent Object Reference") (OtherBodyIndex :type Integer) (bFromSweep :type Boolean) (SweepResult :type "HitResult Structure (by ref)"))
  (goto _label :!via `Open`))

(event `self.Trigger2.OnComponentEndOverlap`
  (params (OverlappedComponent :type "PrimitiveComponent Object Reference") (OtherActor :type "Actor Object Reference") (OtherComp :type "PrimitiveComponent Object Reference") (OtherBodyIndex :type Integer))
  (goto _label :!via `Close`))

(fn `UserConstructionScript`)