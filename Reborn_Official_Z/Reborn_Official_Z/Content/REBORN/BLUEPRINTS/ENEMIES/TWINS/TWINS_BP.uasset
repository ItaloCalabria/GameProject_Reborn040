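; Twins enemy that alternates timed attack and rest phases, started by BEGINALL and mirrored to the IsAttacking_Twins Blackboard key.
; While attacking, its Box repeatedly damages the overlapping player, Edward.
; Edward's taser overlap flashes the mesh and forces a pause, while punch overlaps only hurt it when resting or shocked.
; Health bands drive a self-rechecking lantern color/blink until death; the chase/patrol logic is disconnected.
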(event `PATROL`)

(event `self.ReceiveBeginPlay`
  (bind _edward (`self.Edward`))
  (bind _returnvalue (`PrimitiveComponent.CreateDynamicMaterialInstance` (`self.HP_ENEMY`) 1 "/Game/REBORN/MATERIALS/Lantern_Enemy.Lantern_Enemy" "None"))
  (set `self.Lantern` _returnvalue)
  (`MaterialInstanceDynamic.SetVectorParameterValue` _returnvalue "Light" (struct :`G` 1.0 :`A` 1.0))
  (bind _returnvalue_2 (`PrimitiveComponent.CreateDynamicMaterialInstance` (`self.Mesh`) 0 "/Game/REBORN/MATERIALS/MYASNIK_MAT.MYASNIK_MAT" "None"))
  (set `self.Shock` _returnvalue_2)
  (`MaterialInstanceDynamic.SetVectorParameterValue` :`self` _returnvalue_2 :`ParameterName` "Shock")
  (bind _asedward_blue_print (cast `/Game/REBORN/BLUEPRINTS/Edward_BluePrint` (`GameplayStatics.GetPlayerCharacter` 0)))
  (set `self.Edward` _asedward_blue_print)
  (add `PrimitiveComponent.OnComponentBeginOverlap` (`/Game/REBORN/BLUEPRINTS/Edward_BluePrint.TASER_BOX` _edward) (delegate `OnComponentBeginOverlap_Event_2`))
  (add `PrimitiveComponent.OnComponentBeginOverlap` (`/Game/REBORN/BLUEPRINTS/Edward_BluePrint.Punch_Collision` _edward) (delegate `OnComponentBeginOverlap_Event_0`)))

(event `OnComponentBeginOverlap_Event_2`
  (params (OverlappedComponent :type "PrimitiveComponent Object Reference") (OtherActor :type "Actor Object Reference") (OtherComp :type "PrimitiveComponent Object Reference") (OtherBodyIndex :type Integer) (bFromSweep :type Boolean) (SweepResult :type "HitResult Structure (by ref)"))
  (`self.Shocked`))

(event `BEGINALL`
  (`self.TROCA`)
  (`PrimitiveComponent.SetCollisionResponseToChannel` (`self.Box`) "ECC_WorldStatic" "ECR_Ignore"))

(event `CALL_DEATH`
  ;[1 1 1] CALLDEATH
  (`self.CALLDEATH`)
  (`KismetSystemLibrary.Delay` 1.0)
  (`self.K2_DestroyActor`))

(event `OnComponentBeginOverlap_Event_0`
  (params (OverlappedComponent :type "PrimitiveComponent Object Reference") (OtherActor :type "Actor Object Reference") (OtherComp :type "PrimitiveComponent Object Reference") (OtherBodyIndex :type Integer) (bFromSweep :type Boolean) (SweepResult :type "HitResult Structure (by ref)"))
  (if (or (`self.DECANSANDO`) (`self.CHOCADO`))
    (`self.ReceiveDamage`)
    (set `self.FERIDO` true)
    (`KismetSystemLibrary.Delay` 0.6)
    (set `self.FERIDO` false)
    (`KismetSystemLibrary.PrintString` "MANAÇO")))

(event `Shocked`
  ;[1 1 1] SHOCKED
  (bind (_direction _newtrack_0) (`Timeline|Timeline_0shocktimeline` :!via `PlayFromStart`)
    (:`Update`
      (`MaterialInstanceDynamic.SetVectorParameterValue` (`self.Shock`) "Shock" (`KismetMathLibrary.Conv_VectorToLinearColor` _newtrack_0))
      (set `self.PARA` true)
      (set `self.DECANSANDO` true)
      (bind _output_get (set `self.ATACANDO` false))
      (`BlackboardComponent.SetValueAsBool` (`AIBlueprintHelperLibrary.GetBlackboard` null) "IsAttacking_Twins" _output_get)
      (set `self.CHOCADO` true)
      (`KismetSystemLibrary.Delay` 0.7)
      (set `self.CHOCADO` false)
      (`KismetSystemLibrary.Delay` 4.3)
      (set `self.PARA` false)
      (`self.TROCA`))))

(event `TROCA`
  (bind _output_get (set `self.ATACANDO` true))
  (`BlackboardComponent.SetValueAsBool` (`AIBlueprintHelperLibrary.GetBlackboard` null) "IsAttacking_Twins" _output_get)
  (set `self.DECANSANDO` false)
  (`KismetSystemLibrary.PrintString` "ATACANDO")
  (`KismetSystemLibrary.Delay` 10.0)
  (bind _output_get_2 (set `self.ATACANDO` false))
  (`BlackboardComponent.SetValueAsBool` (`AIBlueprintHelperLibrary.GetBlackboard` null) "IsAttacking_Twins" _output_get_2)
  (set `self.DECANSANDO` true)
  (`KismetSystemLibrary.PrintString` "DESCANSANDO")
  (`KismetSystemLibrary.Delay` 5.0)
  (bind _output_get_3 (set `self.ATACANDO` true))
  (`BlackboardComponent.SetValueAsBool` (`AIBlueprintHelperLibrary.GetBlackboard` null) "IsAttacking_Twins" _output_get_3)
  (`self.TROCA`))

(event `self.Box.OnComponentBeginOverlap`
  (params (OverlappedComponent :type "PrimitiveComponent Object Reference") (OtherActor :type "Actor Object Reference") (OtherComp :type "PrimitiveComponent Object Reference") (OtherBodyIndex :type Integer) (bFromSweep :type Boolean) (SweepResult :type "HitResult Structure (by ref)"))
  (bind _edward (`self.Edward`))
  (cast `/Game/REBORN/BLUEPRINTS/Edward_BluePrint` OtherActor)
  (set `self.CEASE_FIRA` false)
  (if (`self.ATACANDO`)
    (set `/Game/REBORN/BLUEPRINTS/Edward_BluePrint.PersonalDamage` 2 _edward)
    (`/Game/REBORN/BLUEPRINTS/Edward_BluePrint.RECEIVE_DAMAGE` _edward)
    (`self.KEEPDAMAGE`)))

(event `KEEPDAMAGE`
  (if (`self.CEASE_FIRA`)
    _
    (elif (`self.ATACANDO`)
      (`/Game/REBORN/BLUEPRINTS/Edward_BluePrint.RECEIVE_DAMAGE` (`self.Edward`))
      (`KismetSystemLibrary.PrintString` "ai caramab!")
      (`KismetSystemLibrary.Delay` 0.1)
      (`self.KEEPDAMAGE`))))

(event `self.Box.OnComponentEndOverlap`
  (params (OverlappedComponent :type "PrimitiveComponent Object Reference") (OtherActor :type "Actor Object Reference") (OtherComp :type "PrimitiveComponent Object Reference") (OtherBodyIndex :type Integer))
  (cast `/Game/REBORN/BLUEPRINTS/Edward_BluePrint` OtherActor)
  (set `self.CEASE_FIRA` true)
  (`KismetSystemLibrary.PrintString` "CEASE"))

(event `Health100`
  ;[1 1 1] HP_CHECK
  (set `self.FULLHEALTH` false)
  (set `self.Total_HP` 100))

(event `PERFECT_HP`
  ;[1 1 1] HP_CHECK
  (`MaterialInstanceDynamic.SetVectorParameterValue` (`self.Lantern`) "Light" (struct :`G` 6.0 :`A` 1.0))
  (`KismetSystemLibrary.Delay` 0.5)
  (`self.Check_Self`))

(event `Death_Enemy`
  ;[1 1 1] HP_CHECK
  (set `self.DEAD` true)
  (`MaterialInstanceDynamic.SetVectorParameterValue` :`self` (`self.Lantern`) :`ParameterName` "Light")
  (`self.CALLDEATH`)
  (`KismetSystemLibrary.Delay` 0.2)
  (`self.K2_DestroyActor`))

(event `GREAT_HP`
  ;[1 1 1] HP_CHECK
  (bind (_direction _blink_green) (`Timeline|Timeline_0` :!via `PlayFromStart`)
    (:`Update`
      (`MaterialInstanceDynamic.SetVectorParameterValue` (`self.Lantern`) "Light" (`KismetMathLibrary.Conv_VectorToLinearColor` _blink_green))
      (`KismetSystemLibrary.Delay` 0.5)
      (`self.Check_Self`))))

(event `Check_Self`
  ;[1 1 1] HP_CHECK
  (`KismetSystemLibrary.PrintString` (`KismetStringLibrary.Conv_IntToString` (`self.Total_HP`)))
  (if (> (`self.Total_HP`) 100)
    (`self.Health100`)
    (elif (<= (`self.Total_HP`) 0)
      (`self.Death_Enemy`)
      (else
        (switch `int` (`self.HealthSwitch`)
          (:`0`
            (`self.PERFECT_HP`))
          (:`1`
            (`self.GREAT_HP`))
          (:`2`
            (`self.NORMAL_HP`))
          (:`3`
            (`self.BAD_HP`))
          (:`4`
            (`self.HORRIBLE_HP`)))))))

(event `NORMAL_HP`
  ;[1 1 1] HP_CHECK
  (bind (_direction _blink_yellow) (`Timeline|Timeline_1` :!via `PlayFromStart`)
    (:`Update`
      (`MaterialInstanceDynamic.SetVectorParameterValue` (`self.Lantern`) "Light" (`KismetMathLibrary.Conv_VectorToLinearColor` _blink_yellow))
      (`KismetSystemLibrary.Delay` 0.5)
      (`self.Check_Self`))))

(event `BAD_HP`
  ;[1 1 1] HP_CHECK
  (bind (_direction _blink_red) (`Timeline|Timeline_2` :!via `PlayFromStart`)
    (:`Update`
      (`MaterialInstanceDynamic.SetVectorParameterValue` (`self.Lantern`) "Light" (`KismetMathLibrary.Conv_VectorToLinearColor` _blink_red))
      (`KismetSystemLibrary.Delay` 0.5)
      (`self.Check_Self`))))

(event `HORRIBLE_HP`
  ;[1 1 1] HP_CHECK
  (`MaterialInstanceDynamic.SetVectorParameterValue` (`self.Lantern`) "Light" (struct :`R` 6.0 :`A` 1.0))
  (`KismetSystemLibrary.Delay` 0.5)
  (`self.Check_Self`))

(event `ReceiveDamage`
  (bind _total_hp (`self.Total_HP`))
  ;[1 1 1] HP_CHECK
  (set `self.Total_HP` (- (`self.Total_HP`) (`self.Damage_Rate`)))
  (`self.Check_Self`)
  (if (`KismetMathLibrary.InRange_IntInt` _total_hp 96 100)
    (set `self.HealthSwitch` 0)
    (`self.Check_Self`)
    (elif (`KismetMathLibrary.InRange_IntInt` _total_hp 66 95)
      (set `self.HealthSwitch` 1)
      (`self.Check_Self`)
      (elif (`KismetMathLibrary.InRange_IntInt` _total_hp 36 65)
        (set `self.HealthSwitch` 2)
        (`self.Check_Self`)
        (elif (`KismetMathLibrary.InRange_IntInt` _total_hp 6 35)
          (set `self.HealthSwitch` 3)
          (`self.Check_Self`)
          (elif (`KismetMathLibrary.InRange_IntInt` _total_hp 1 5)
            (set `self.HealthSwitch` 4)
            (`self.Check_Self`)))))))

(fn `UserConstructionScript`)