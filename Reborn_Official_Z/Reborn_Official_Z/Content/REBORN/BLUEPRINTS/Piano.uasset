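; Piano puzzle Blueprint where number keys 1–7 play notes to enter a code, with input disabled at BeginPlay.
; Each press animates the piano, advances the Roleta indicator and appends a digit until the TotalDigitos countdown ends, then compares against RespostaCerta.
; A match plays a success sequence, sets Correct and returns the camera, while a mismatch resets with discordant notes after a short delay.
; E also triggers the camera return.
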(event `self.ReceiveBeginPlay`
  ;[1 1 1] EVENT BEGIN PLAY
  (`self.DisableInput` (`GameplayStatics.GetPlayerController` 0) null))

(event `Key|One` :consume false
  (params (Key :type "Key Structure"))
  (:`Pressed`
    (set `self.Key` 0)
    (`self.Check_Click`)))

(event `Key|Two` :consume false
  (params (Key :type "Key Structure"))
  (:`Pressed`
    (set `self.Key` 1)
    (`self.Check_Click`)))

(event `Check_Click`
  (`self.Tecla` (`self.Key`)))

(event `LightAnswer`
  (switch `int` (`self.TotalDigitos`)
    (:`0`
      (`SkeletalMeshComponent.PlayAnimation` (`self.Roleta`) "/Game/untitled_category/untitled_asset/animations/rp0.rp0" false)
      (`GameplayStatics.PlaySound2D` "/Game/REBORN/SOUNDS/LIGHT_CLICK.LIGHT_CLICK" 1.0 1.0 0.0 null null))
    (:`1`
      (`SkeletalMeshComponent.PlayAnimation` (`self.Roleta`) "/Game/untitled_category/untitled_asset/animations/rp6.rp6" false)
      (`GameplayStatics.PlaySound2D` "/Game/REBORN/SOUNDS/LIGHT_CLICK.LIGHT_CLICK" 1.0 1.0 0.0 null null))
    (:`2`
      (`SkeletalMeshComponent.PlayAnimation` (`self.Roleta`) "/Game/untitled_category/untitled_asset/animations/rp5.rp5" false)
      (`GameplayStatics.PlaySound2D` "/Game/REBORN/SOUNDS/LIGHT_CLICK.LIGHT_CLICK" 1.0 1.0 0.0 null null))
    (:`3`
      (`SkeletalMeshComponent.PlayAnimation` (`self.Roleta`) "/Game/untitled_category/untitled_asset/animations/rp4.rp4" false)
      (`GameplayStatics.PlaySound2D` "/Game/REBORN/SOUNDS/LIGHT_CLICK.LIGHT_CLICK" 1.0 1.0 0.0 null null))
    (:`4`
      (`SkeletalMeshComponent.PlayAnimation` (`self.Roleta`) "/Game/untitled_category/untitled_asset/animations/rp3.rp3" false)
      (`GameplayStatics.PlaySound2D` "/Game/REBORN/SOUNDS/LIGHT_CLICK.LIGHT_CLICK" 1.0 1.0 0.0 null null))
    (:`5`
      (`SkeletalMeshComponent.PlayAnimation` (`self.Roleta`) "/Game/untitled_category/untitled_asset/animations/rp2.rp2" false)
      (`GameplayStatics.PlaySound2D` "/Game/REBORN/SOUNDS/LIGHT_CLICK.LIGHT_CLICK" 1.0 1.0 0.0 null null))
    (:`6`
      (`SkeletalMeshComponent.PlayAnimation` (`self.Roleta`) "/Game/untitled_category/untitled_asset/animations/rp1.rp1" false)
      (`GameplayStatics.PlaySound2D` "/Game/REBORN/SOUNDS/LIGHT_CLICK.LIGHT_CLICK" 1.0 1.0 0.0 null null))))

(event `Key|Three` :consume false
  (params (Key :type "Key Structure"))
  (:`Pressed`
    (set `self.Key` 2)
    (`self.Check_Click`)))

(event `Key|Four` :consume false
  (params (Key :type "Key Structure"))
  (:`Pressed`
    (set `self.Key` 3)
    (`self.Check_Click`)))

(event `Key|Five` :consume false
  (params (Key :type "Key Structure"))
  (:`Pressed`
    (set `self.Key` 4)
    (`self.Check_Click`)))

(event `ChecarTecla`
  (params (component :type "PrimitiveComponent Object Reference")))

(event `Key|Six` :consume false
  (params (Key :type "Key Structure"))
  (:`Pressed`
    (set `self.Key` 5)
    (`self.Check_Click`)))

(event `Key|Seven` :consume false
  (params (Key :type "Key Structure"))
  (:`Pressed`
    (set `self.Key` 6)
    (`self.Check_Click`)))

(event `Key|E`
  (params (Key :type "Key Structure"))
  (:`Pressed`
    (`self.RetornoCamera`)))

(event `Acertou`
  (`self.DisableInput` (`GameplayStatics.GetPlayerController` 0))
  (`KismetSystemLibrary.Delay` 0.5)
  (`SkeletalMeshComponent.PlayAnimation` (`self.Piano`) "/Game/untitled_category/untitled_asset/animations/C_Montage.C_Montage" false)
  (`GameplayStatics.PlaySound2D` "/Game/REBORN/SOUNDS/piano-c_C_major.piano-c_C_major" 1.0 1.0 0.0 null null)
  (`KismetSystemLibrary.Delay` 0.1)
  (`SkeletalMeshComponent.PlayAnimation` (`self.Piano`) "/Game/untitled_category/untitled_asset/animations/G_Montage.G_Montage" false)
  (`GameplayStatics.PlaySound2D` "/Game/REBORN/SOUNDS/piano-g_G_major.piano-g_G_major" 1.0 1.0 0.0 null null)
  (`KismetSystemLibrary.Delay` 0.5)
  (`SkeletalMeshComponent.PlayAnimation` (`self.Roleta`) "/Game/untitled_category/untitled_asset/animations/rpBEDEAD.rpBEDEAD" false)
  (`GameplayStatics.PlaySound2D` "/Game/REBORN/SOUNDS/LIGHT_CLICK.LIGHT_CLICK" 1.0 1.0 0.0 null null)
  (`KismetSystemLibrary.Delay` 2.0)
  (set `self.Correct` true)
  (`self.RetornoCamera`))

(event `RetornoCamera`
  (`self.BackCAMERA`))

(event `Errou`
  (`GameplayStatics.PlaySound2D` "/Game/REBORN/SOUNDS/piano-a_A_major.piano-a_A_major" 1.0 1.0 0.0 null null)
  (`GameplayStatics.PlaySound2D` "/Game/REBORN/SOUNDS/piano-e_E_major.piano-e_E_major" 1.0 1.0 0.0 null null)
  (`GameplayStatics.PlaySound2D` "/Game/REBORN/SOUNDS/piano-f_F_major.piano-f_F_major" 1.0 1.0 0.0 null null)
  (`GameplayStatics.PlaySound2D` "/Game/REBORN/SOUNDS/piano-b_B_major.piano-b_B_major" 1.0 1.0 0.0 null null)
  (`GameplayStatics.PlaySound2D` "/Game/REBORN/SOUNDS/piano-d_D_major.piano-d_D_major" 1.0 1.0 0.0 null null)
  (`GameplayStatics.PlaySound2D` "/Game/REBORN/SOUNDS/LOCKSWITCH.LOCKSWITCH" 1.0 1.0 0.0 null null))

(event `ResetarTexto`
  ;[1 1 1] Reset
  (set `self.TotalDigitos` 6)
  (set `self.textoDigitado` "")
  (`SkeletalMeshComponent.PlayAnimation` (`self.Roleta`) "/Game/untitled_category/untitled_asset/animations/rp0.rp0" false))

(fn `UserConstructionScript`)