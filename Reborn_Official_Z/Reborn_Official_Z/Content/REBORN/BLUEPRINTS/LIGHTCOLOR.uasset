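; Blueprint with a point light whose color changes through keyboard input.
; Key press events for J, K, L and P each call SetLightColor on the PointLight with a fixed color: green, red, blue or white.
; The keys are bound directly in the event graph, and the construction script is empty.
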(event `Key|J` :consume false
  (params (Key :type "Key Structure"))
  (:`Pressed`
    (`LightComponent.SetLightColor` (`self.PointLight`) (struct :`G` 1.0 :`A` 1.0) true)))

(event `Key|K` :consume false
  (params (Key :type "Key Structure"))
  (:`Pressed`
    (`LightComponent.SetLightColor` (`self.PointLight`) (struct :`R` 1.0 :`A` 1.0) true)))

(event `Key|L` :consume false
  (params (Key :type "Key Structure"))
  (:`Pressed`
    (`LightComponent.SetLightColor` (`self.PointLight`) (struct :`B` 1.0 :`A` 1.0) true)))

(event `Key|P` :consume false
  (params (Key :type "Key Structure"))
  (:`Pressed`
    (`LightComponent.SetLightColor` (`self.PointLight`) (struct :`R` 1.0 :`G` 1.0 :`B` 1.0 :`A` 1.0) true)))

(fn `UserConstructionScript`)