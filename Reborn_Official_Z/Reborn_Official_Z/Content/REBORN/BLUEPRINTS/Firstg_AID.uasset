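; First aid cabinet pickup that restores the player's health.
; When Edward enters the outer trigger below full HP, the cabinet plays its hinge animation and open sound once.
; An inner trigger gates the Action input, which smoothly turns Edward toward the cabinet via a timeline yaw lerp.
; He then plays CATCH, and after a short delay the HP component and inner trigger are destroyed and ReceiveHP is called.
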(event `self.ReceiveBeginPlay`
  (bind _asedward_blue_print (cast `/Game/REBORN/BLUEPRINTS/Edward_BluePrint` (`GameplayStatics.GetPlayerCharacter` 0)))
  (set `self.Edward` _asedward_blue_print))

(event `self.Trigger.OnComponentBeginOverlap`
  (params (OverlappedComponent :type "PrimitiveComponent Object Reference") (OtherActor :type "Actor Object Reference") (OtherComp :type "PrimitiveComponent Object Reference") (OtherBodyIndex :type Integer) (bFromSweep :type Boolean) (SweepResult :type "HitResult Structure (by ref)"))
  (if (not (== (`/Game/REBORN/BLUEPRINTS/Edward_BluePrint.HP` (`self.Edward`)) 100))
    (`SkeletalMeshComponent.PlayAnimation` (`self.SkeletalMesh`) "/Game/untitled_category/untitled_asset/animations/Hinge.Hinge" false)
    (`GameplayStatics.PlaySound2D` "/Game/REBORN/SOUNDS/CABINET_OPEN.CABINET_OPEN" 1.0 1.0 0.0 null null)
    (set `PrimitiveComponent.bGenerateOverlapEvents` false (`self.Trigger`))))

(event `InputAction|Action` :consume false
  (params (Key :type "Key Structure"))
  (bind _edward (`self.Edward`))
  (bind _edward_2 (`self.Edward`))
  (bind (_returnvalue_roll _returnvalue_pitch _returnvalue_yaw) (`KismetMathLibrary.BreakRotator` (`KismetMathLibrary.FindLookAtRotation` (`self.K2_GetActorLocation` _edward_2) (`self.K2_GetActorLocation`))))
  (:`Pressed`
    (`/Engine/EditorBlueprintResources/StandardMacros.Gate` true :!label _label
      (:`Exit`
        (if (not (== (`/Game/REBORN/BLUEPRINTS/Edward_BluePrint.HP` (`self.Edward`)) 100))
          (set `self.Rotation` (`self.K2_GetActorRotation` _edward_2))
          (bind (_direction _newtrack_0) (`Timeline|Timeline_0` :!via `PlayFromStart`)
            (:`Update`
              (`self.K2_SetActorRotation` _edward_2 (`KismetMathLibrary.RLerp` (`self.Rotation`) (`KismetMathLibrary.MakeRotator` 0.0 0.0 _returnvalue_yaw) _newtrack_0 true) false))
            (:`Finished`
              (`/Engine/EditorBlueprintResources/StandardMacros.DoOnce` false
                (:`Completed`
                  (`/Game/REBORN/BLUEPRINTS/Edward_BluePrint.CATCH` _edward)
                  (`KismetSystemLibrary.Delay` 0.5)
                  (`GameplayStatics.PlaySound2D` "/Game/REBORN/SOUNDS/ACTUAL_HP.ACTUAL_HP" 1.0 1.0 0.0 null null)
                  (`ActorComponent.K2_DestroyComponent` (`self.HP`))
                  (`ActorComponent.K2_DestroyComponent` (`self.Trigger2`))
                  (`/Game/REBORN/BLUEPRINTS/Edward_BluePrint.Receive_HP` _edward)
                  (`KismetSystemLibrary.PrintString` "Hello"))))))))))

(event `self.Trigger2.OnComponentBeginOverlap`
  (params (OverlappedComponent :type "PrimitiveComponent Object Reference") (OtherActor :type "Actor Object Reference") (OtherComp :type "PrimitiveComponent Object Reference") (OtherBodyIndex :type Integer) (bFromSweep :type Boolean) (SweepResult :type "HitResult Structure (by ref)"))
  (goto _label :!via `Open`))

(event `self.Trigger2.OnComponentEndOverlap`
  (params (OverlappedComponent :type "PrimitiveComponent Object Reference") (OtherActor :type "Actor Object Reference") (OtherComp :type "PrimitiveComponent Object Reference") (OtherBodyIndex :type Integer))
  (goto _label :!via `Close`))

(fn `UserConstructionScript`)