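; Static camera actor that takes over the first player's view when its StartCamera trigger is overlapped.
; On BeginPlay it caches the player character as an Edward_BluePrint reference.
; Overlap blends the player controller's view target to this actor over BlendTime.
; The Edward cast on the overlapping actor does not gate the switch, and nothing here restores the previous view.
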(event `self.ReceiveBeginPlay`
  (bind _asedward_blue_print (cast `/Game/REBORN/BLUEPRINTS/Edward_BluePrint` (`GameplayStatics.GetPlayerCharacter` 0)))
  (set `self.Edward` _asedward_blue_print))

(event `self.StartCamera.OnComponentBeginOverlap`
  (params (OverlappedComponent :type "PrimitiveComponent Object Reference") (OtherActor :type "Actor Object Reference") (OtherComp :type "PrimitiveComponent Object Reference") (OtherBodyIndex :type Integer) (bFromSweep :type Boolean) (SweepResult :type "HitResult Structure (by ref)"))
  (cast `/Game/REBORN/BLUEPRINTS/Edward_BluePrint` OtherActor
    (:`then`
      _)
    (:`CastFailed`
      (set `self.Edward` (`self.Edward`))))
  (`PlayerController.SetViewTargetWithBlend` (`GameplayStatics.GetPlayerController` 0) self (`self.BlendTime`) "VTBlend_Linear" 0.0 false))

(fn `UserConstructionScript`)