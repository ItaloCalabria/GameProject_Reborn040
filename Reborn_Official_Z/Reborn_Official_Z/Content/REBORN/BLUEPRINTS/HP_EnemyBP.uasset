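; Enemy health Blueprint that tracks HP and displays it through the color of a lantern material.
; ReceiveDamage subtracts DamageRate and maps HP into five LightSwitch tiers, from steady green through timeline-driven green, yellow and red blinks to steady red.
; Check_Self caps HP at 100, routes to the tier's light event, which re-checks after a delay, or triggers death.
; Death darkens the lantern and calls the CALLDEATH dispatcher.
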(event `self.ReceiveBeginPlay`
  (bind _returnvalue (`PrimitiveComponent.CreateDynamicMaterialInstance` (`self.HP_Enemy`) 1 "/Game/REBORN/MATERIALS/Lantern_Enemy.Lantern_Enemy" "None"))
  (set `self.Enemy_Lantern` _returnvalue)
  (`MaterialInstanceDynamic.SetVectorParameterValue` _returnvalue "Light" (struct :`G` 6.0 :`A` 1.0)))

(event `Health100`
  (set `self.HP_Complete` true)
  (set `self.Enemy_HP` 100))

(event `PERFECT_HP`
  (`MaterialInstanceDynamic.SetVectorParameterValue` (`self.Enemy_Lantern`) "Light" (struct :`G` 6.0 :`A` 1.0))
  (`KismetSystemLibrary.Delay` 0.5)
  (`self.Check_Self`))

(event `Death_Enemy`
  (set `self.Dead` true)
  (`MaterialInstanceDynamic.SetVectorParameterValue` :`self` (`self.Enemy_Lantern`) :`ParameterName` "Light")
  (`self.CALL_DEATH`))

(event `GREAT_HP`
  (bind (_direction _blink_green) (`Timeline|Timeline_0` :!via `PlayFromStart`)
    (:`Update`
      (`MaterialInstanceDynamic.SetVectorParameterValue` (`self.Enemy_Lantern`) "Light" (`KismetMathLibrary.Conv_VectorToLinearColor` _blink_green))
      (`KismetSystemLibrary.Delay` 0.5)
      (`self.Check_Self`))))

(event `Check_Self`
  (`KismetSystemLibrary.PrintString` (`KismetStringLibrary.Conv_IntToString` (`self.Enemy_HP`)))
  (if (> (`self.Enemy_HP`) 100)
    (`self.Health100`)
    (elif (<= (`self.Enemy_HP`) 0)
      (`self.Death_Enemy`)
      (else
        (switch `int` (`self.Light_Switch`)
          (:`0`
            (`self.PERFECT_HP`))
          (:`1`
            (`self.GREAT_HP`))
          (:`2`
            (`self.NORMAL_HP`))
          (:`3`
            (`self.BAD_HP`))
          (:`4`
            (`self.HORRIBLE_HP`)))))))

(event `NORMAL_HP`
  (bind (_direction _blink_yellow) (`Timeline|Timeline_1` :!via `PlayFromStart`)
    (:`Update`
      (`MaterialInstanceDynamic.SetVectorParameterValue` (`self.Enemy_Lantern`) "Light" (`KismetMathLibrary.Conv_VectorToLinearColor` _blink_yellow))
      (`KismetSystemLibrary.Delay` 0.5)
      (`self.Check_Self`))))

(event `BAD_HP`
  (bind (_direction _blink_red) (`Timeline|Timeline_2` :!via `PlayFromStart`)
    (:`Update`
      (`MaterialInstanceDynamic.SetVectorParameterValue` (`self.Enemy_Lantern`) "Light" (`KismetMathLibrary.Conv_VectorToLinearColor` _blink_red))
      (`KismetSystemLibrary.Delay` 0.5)
      (`self.Check_Self`))))

(event `HORRIBLE_HP`
  (`MaterialInstanceDynamic.SetVectorParameterValue` (`self.Enemy_Lantern`) "Light" (struct :`R` 6.0 :`A` 1.0))
  (`KismetSystemLibrary.Delay` 0.5)
  (`self.Check_Self`))

(event `ReceiveDamage`
  (bind _enemy_hp (`self.Enemy_HP`))
  (set `self.Enemy_HP` (- (`self.Enemy_HP`) (`self.Damage_Rate`)))
  (`self.Check_Self`)
  (if (`KismetMathLibrary.InRange_IntInt` _enemy_hp 96 100)
    (set `self.Light_Switch` 0)
    (`self.Check_Self`)
    (elif (`KismetMathLibrary.InRange_IntInt` _enemy_hp 66 95)
      (set `self.Light_Switch` 1)
      (`self.Check_Self`)
      (elif (`KismetMathLibrary.InRange_IntInt` _enemy_hp 36 65)
        (set `self.Light_Switch` 2)
        (`self.Check_Self`)
        (elif (`KismetMathLibrary.InRange_IntInt` _enemy_hp 6 35)
          (set `self.Light_Switch` 3)
          (`self.Check_Self`)
          (elif (`KismetMathLibrary.InRange_IntInt` _enemy_hp 1 5)
            (set `self.Light_Switch` 4)
            (`self.Check_Self`)))))))

(fn `UserConstructionScript`)