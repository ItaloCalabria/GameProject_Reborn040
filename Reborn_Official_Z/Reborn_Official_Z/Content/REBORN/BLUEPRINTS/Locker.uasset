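; Six-dial combination lock puzzle that the player works with the mouse.
; Left and right clicks cycle the selected dial, and the wheel steps its digit through 0–5 using one Switch1 counter shared by all dials.
; Each turn animates the dial and joins the six answers to compare with RightAnswer.
; A match plays the unlock animation and sound, then calls Correct after a short delay, while E calls CallBack to exit.
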(event `Get_Out`
  (`self.Call_Back`))

(event `Correct_Password`
  (`SkeletalMeshComponent.PlayAnimation` (`self.LOCKER`) "/Game/untitled_category/untitled_asset/animations/LockerFinal.LockerFinal" false)
  (`GameplayStatics.PlaySound2D` "/Game/REBORN/SOUNDS/OPENLOCK.OPENLOCK" 1.0 1.0 0.0 null null)
  (`KismetSystemLibrary.Delay` 0.5)
  (`self.Correct`))

(event `Key|RightMouseButton`
  (params (Key :type "Key Structure"))
  (bind _locker (`self.LOCKER`))
  (bind _mainswitch (`self.MainSwitch`))
  (:`Pressed`
    (set `self.MainSwitch` (+ _mainswitch 1))
    (if (> _mainswitch 5)
      (set `self.MainSwitch` 0))
    (switch `int` (`self.MainSwitch`) :!label _label
      (:`0`
        (`SkeletalMeshComponent.PlayAnimation` _locker "/Game/untitled_category/untitled_asset/animations/LR1.LR1" false)
        (`GameplayStatics.PlaySound2D` "/Game/REBORN/SOUNDS/LOCKSWITCH.LOCKSWITCH" 1.0 1.0 0.0 null null))
      (:`1`
        (`SkeletalMeshComponent.PlayAnimation` _locker "/Game/untitled_category/untitled_asset/animations/LR2.LR2" false)
        (`GameplayStatics.PlaySound2D` "/Game/REBORN/SOUNDS/LOCKSWITCH.LOCKSWITCH" 1.0 1.0 0.0 null null))
      (:`2`
        (`SkeletalMeshComponent.PlayAnimation` _locker "/Game/untitled_category/untitled_asset/animations/LR3.LR3" false)
        (`GameplayStatics.PlaySound2D` "/Game/REBORN/SOUNDS/LOCKSWITCH.LOCKSWITCH" 1.0 1.0 0.0 null null))
      (:`3`
        (`SkeletalMeshComponent.PlayAnimation` _locker "/Game/untitled_category/untitled_asset/animations/LR4.LR4" false)
        (`GameplayStatics.PlaySound2D` "/Game/REBORN/SOUNDS/LOCKSWITCH.LOCKSWITCH" 1.0 1.0 0.0 null null))
      (:`4`
        (`SkeletalMeshComponent.PlayAnimation` _locker "/Game/untitled_category/untitled_asset/animations/LR5.LR5" false)
        (`GameplayStatics.PlaySound2D` "/Game/REBORN/SOUNDS/LOCKSWITCH.LOCKSWITCH" 1.0 1.0 0.0 null null))
      (:`5`
        (`SkeletalMeshComponent.PlayAnimation` _locker "/Game/untitled_category/untitled_asset/animations/LR6.LR6" false)
        (`GameplayStatics.PlaySound2D` "/Game/REBORN/SOUNDS/LOCKSWITCH.LOCKSWITCH" 1.0 1.0 0.0 null null)))))

(event `Check_Answer`
  (set `self.Answering` (`KismetStringLibrary.Concat_StrStr` (`self.Answer1`) (`self.Answer2`) (`self.Answer3`) (`self.Answer4`) (`self.Answer5`) (`self.Naswer6`)))
  (if (`KismetStringLibrary.EqualEqual_StrStr` (`self.Answering`) (`self.RightAnswer`))
    (`self.Correct_Password`)))

(event `Key|E`
  (params (Key :type "Key Structure"))
  (:`Pressed`
    (`self.Get_Out`)))

(event `Key|LeftMouseButton`
  (params (Key :type "Key Structure"))
  (bind _mainswitch (`self.MainSwitch`))
  (:`Pressed`
    (set `self.MainSwitch` (- _mainswitch 1))
    (if (< _mainswitch 0)
      (set `self.MainSwitch` (+ (`self.MainSwitch`) 6))
      (goto _label)
      (else
        (goto _label)))))

(event `Key|MouseScrollUp` :consume false
  (params (Key :type "Key Structure"))
  (bind _r6 (`self.R6`))
  (bind _mainswitch (`self.MainSwitch`))
  (bind _switch1 (`self.switch1`))
  (bind _switch1_2 (`self.switch1`))
  (bind _r1 (`self.R1`))
  (bind _switch1_3 (`self.switch1`))
  (bind _r2 (`self.R2`))
  (bind _switch1_4 (`self.switch1`))
  (bind _r5 (`self.R5`))
  (bind _switch1_5 (`self.switch1`))
  (bind _r3 (`self.R3`))
  (bind _switch1_6 (`self.switch1`))
  (bind _r4 (`self.R4`))
  (:`Pressed`
    (if (== _mainswitch 0)
      ;[1 1 1] 1
      (bind _output_get (set `self.switch1` (- _switch1 1)))
      (if (< _switch1 0)
        (set `self.switch1` (+ _switch1 6)))
      (`KismetSystemLibrary.PrintString` (`KismetStringLibrary.Conv_IntToString` _output_get))
      (switch `int` (`self.switch1`) :!label _label_2
        (:`0`
          (`SkeletalMeshComponent.PlayAnimation` _r1 "/Game/untitled_category/untitled_asset/animations/RLR1.RLR1" false)
          (`GameplayStatics.PlaySound2D` "/Game/REBORN/SOUNDS/LOCKSWITCH.LOCKSWITCH" 1.0 1.0 0.0 null null)
          (set `self.Answer1` "0")
          (`self.Check_Answer`))
        (:`1`
          (`SkeletalMeshComponent.PlayAnimation` _r1 "/Game/untitled_category/untitled_asset/animations/RLR2.RLR2" false)
          (`GameplayStatics.PlaySound2D` "/Game/REBORN/SOUNDS/LOCKSWITCH.LOCKSWITCH" 1.0 1.0 0.0 null null)
          (set `self.Answer1` "1")
          (`self.Check_Answer`))
        (:`2`
          (`SkeletalMeshComponent.PlayAnimation` _r1 "/Game/untitled_category/untitled_asset/animations/RLR3.RLR3" false)
          (`GameplayStatics.PlaySound2D` "/Game/REBORN/SOUNDS/LOCKSWITCH.LOCKSWITCH" 1.0 1.0 0.0 null null)
          (set `self.Answer1` "2")
          (`self.Check_Answer`))
        (:`3`
          (`SkeletalMeshComponent.PlayAnimation` _r1 "/Game/untitled_category/untitled_asset/animations/RLR4.RLR4" false)
          (`GameplayStatics.PlaySound2D` "/Game/REBORN/SOUNDS/LOCKSWITCH.LOCKSWITCH" 1.0 1.0 0.0 null null)
          (set `self.Answer1` "3")
          (`self.Check_Answer`))
        (:`4`
          (`SkeletalMeshComponent.PlayAnimation` _r1 "/Game/untitled_category/untitled_asset/animations/RLR5.RLR5" false)
          (`GameplayStatics.PlaySound2D` "/Game/REBORN/SOUNDS/LOCKSWITCH.LOCKSWITCH" 1.0 1.0 0.0 null null)
          (set `self.Answer1` "4")
          (`self.Check_Answer`))
        (:`5`
          (`SkeletalMeshComponent.PlayAnimation` _r1 "/Game/untitled_category/untitled_asset/animations/RLR6.RLR6" false)
          (`GameplayStatics.PlaySound2D` "/Game/REBORN/SOUNDS/LOCKSWITCH.LOCKSWITCH" 1.0 1.0 0.0 null null)
          (set `self.Answer1` "5")
          (`self.Check_Answer`)))
      (elif (== _mainswitch 1)
        ;[1 1 1] 2
        (bind _output_get_2 (set `self.switch1` (- _switch1_3 1)))
        (if (< _switch1_3 0)
          (set `self.switch1` (+ _switch1_3 6)))
        (`KismetSystemLibrary.PrintString` (`KismetStringLibrary.Conv_IntToString` _output_get_2))
        (switch `int` (`self.switch1`) :!label _label_3
          (:`0`
            (`SkeletalMeshComponent.PlayAnimation` _r2 "/Game/untitled_category/untitled_asset/animations/RLR1.RLR1" false)
            (`GameplayStatics.PlaySound2D` "/Game/REBORN/SOUNDS/LOCKSWITCH.LOCKSWITCH" 1.0 1.0 0.0 null null)
            (set `self.Answer2` "0")
            (`self.Check_Answer`))
          (:`1`
            (`SkeletalMeshComponent.PlayAnimation` _r2 "/Game/untitled_category/untitled_asset/animations/RLR2.RLR2" false)
            (`GameplayStatics.PlaySound2D` "/Game/REBORN/SOUNDS/LOCKSWITCH.LOCKSWITCH" 1.0 1.0 0.0 null null)
            (set `self.Answer2` "1")
            (`self.Check_Answer`))
          (:`2`
            (`SkeletalMeshComponent.PlayAnimation` _r2 "/Game/untitled_category/untitled_asset/animations/RLR3.RLR3" false)
            (`GameplayStatics.PlaySound2D` "/Game/REBORN/SOUNDS/LOCKSWITCH.LOCKSWITCH" 1.0 1.0 0.0 null null)
            (set `self.Answer2` "2")
            (`self.Check_Answer`))
          (:`3`
            (`SkeletalMeshComponent.PlayAnimation` _r2 "/Game/untitled_category/untitled_asset/animations/RLR4.RLR4" false)
            (`GameplayStatics.PlaySound2D` "/Game/REBORN/SOUNDS/LOCKSWITCH.LOCKSWITCH" 1.0 1.0 0.0 null null)
            (set `self.Answer2` "3")
            (`self.Check_Answer`))
          (:`4`
            (`SkeletalMeshComponent.PlayAnimation` _r2 "/Game/untitled_category/untitled_asset/animations/RLR5.RLR5" false)
            (`GameplayStatics.PlaySound2D` "/Game/REBORN/SOUNDS/LOCKSWITCH.LOCKSWITCH" 1.0 1.0 0.0 null null)
            (set `self.Answer2` "4")
            (`self.Check_Answer`))
          (:`5`
            (`SkeletalMeshComponent.PlayAnimation` _r2 "/Game/untitled_category/untitled_asset/animations/RLR6.RLR6" false)
            (`GameplayStatics.PlaySound2D` "/Game/REBORN/SOUNDS/LOCKSWITCH.LOCKSWITCH" 1.0 1.0 0.0 null null)
            (set `self.Answer2` "5")
            (`self.Check_Answer`)))
        (elif (== _mainswitch 2)
          ;[1 1 1] 3
          (bind _output_get_3 (set `self.switch1` (- _switch1_5 1)))
          (if (< _switch1_5 0)
            (set `self.switch1` (+ _switch1_5 6)))
          (`KismetSystemLibrary.PrintString` (`KismetStringLibrary.Conv_IntToString` _output_get_3))
          (switch `int` (`self.switch1`) :!label _label_4
            (:`0`
              (`SkeletalMeshComponent.PlayAnimation` _r3 "/Game/untitled_category/untitled_asset/animations/RLR1.RLR1" false)
              (`GameplayStatics.PlaySound2D` "/Game/REBORN/SOUNDS/LOCKSWITCH.LOCKSWITCH" 1.0 1.0 0.0 null null)
              (set `self.Answer3` "0")
              (`self.Check_Answer`))
            (:`1`
              (`SkeletalMeshComponent.PlayAnimation` _r3 "/Game/untitled_category/untitled_asset/animations/RLR2.RLR2" false)
              (`GameplayStatics.PlaySound2D` "/Game/REBORN/SOUNDS/LOCKSWITCH.LOCKSWITCH" 1.0 1.0 0.0 null null)
              (set `self.Answer3` "1")
              (`self.Check_Answer`))
            (:`2`
              (`SkeletalMeshComponent.PlayAnimation` _r3 "/Game/untitled_category/untitled_asset/animations/RLR3.RLR3" false)
              (`GameplayStatics.PlaySound2D` "/Game/REBORN/SOUNDS/LOCKSWITCH.LOCKSWITCH" 1.0 1.0 0.0 null null)
              (set `self.Answer3` "2")
              (`self.Check_Answer`))
            (:`3`
              (`SkeletalMeshComponent.PlayAnimation` _r3 "/Game/untitled_category/untitled_asset/animations/RLR4.RLR4" false)
              (`GameplayStatics.PlaySound2D` "/Game/REBORN/SOUNDS/LOCKSWITCH.LOCKSWITCH" 1.0 1.0 0.0 null null)
              (set `self.Answer3` "3")
              (`self.Check_Answer`))
            (:`4`
              (`SkeletalMeshComponent.PlayAnimation` _r3 "/Game/untitled_category/untitled_asset/animations/RLR5.RLR5" false)
              (`GameplayStatics.PlaySound2D` "/Game/REBORN/SOUNDS/LOCKSWITCH.LOCKSWITCH" 1.0 1.0 0.0 null null)
              (set `self.Answer3` "4")
              (`self.Check_Answer`))
            (:`5`
              (`SkeletalMeshComponent.PlayAnimation` _r3 "/Game/untitled_category/untitled_asset/animations/RLR6.RLR6" false)
              (`GameplayStatics.PlaySound2D` "/Game/REBORN/SOUNDS/LOCKSWITCH.LOCKSWITCH" 1.0 1.0 0.0 null null)
              (set `self.Answer3` "5")
              (`self.Check_Answer`)))
          (elif (== _mainswitch 3)
            ;[1 1 1] 4
            (bind _output_get_4 (set `self.switch1` (- _switch1_6 1)))
            (if (< _switch1_6 0)
              (set `self.switch1` (+ _switch1_6 6)))
            (`KismetSystemLibrary.PrintString` (`KismetStringLibrary.Conv_IntToString` _output_get_4))
            (switch `int` (`self.switch1`) :!label _label_5
              (:`0`
                (`SkeletalMeshComponent.PlayAnimation` _r4 "/Game/untitled_category/untitled_asset/animations/RLR1.RLR1" false)
                (`GameplayStatics.PlaySound2D` "/Game/REBORN/SOUNDS/LOCKSWITCH.LOCKSWITCH" 1.0 1.0 0.0 null null)
                (set `self.Answer4` "0")
                (`self.Check_Answer`))
              (:`1`
                (`SkeletalMeshComponent.PlayAnimation` _r4 "/Game/untitled_category/untitled_asset/animations/RLR2.RLR2" false)
                (`GameplayStatics.PlaySound2D` "/Game/REBORN/SOUNDS/LOCKSWITCH.LOCKSWITCH" 1.0 1.0 0.0 null null)
                (set `self.Answer4` "1")
                (`self.Check_Answer`))
              (:`2`
                (`SkeletalMeshComponent.PlayAnimation` _r4 "/Game/untitled_category/untitled_asset/animations/RLR3.RLR3" false)
                (`GameplayStatics.PlaySound2D` "/Game/REBORN/SOUNDS/LOCKSWITCH.LOCKSWITCH" 1.0 1.0 0.0 null null)
                (set `self.Answer4` "2")
                (`self.Check_Answer`))
              (:`3`
                (`SkeletalMeshComponent.PlayAnimation` _r4 "/Game/untitled_category/untitled_asset/animations/RLR4.RLR4" false)
                (`GameplayStatics.PlaySound2D` "/Game/REBORN/SOUNDS/LOCKSWITCH.LOCKSWITCH" 1.0 1.0 0.0 null null)
                (set `self.Answer4` "3")
                (`self.Check_Answer`))
              (:`4`
                (`SkeletalMeshComponent.PlayAnimation` _r4 "/Game/untitled_category/untitled_asset/animations/RLR5.RLR5" false)
                (`GameplayStatics.PlaySound2D` "/Game/REBORN/SOUNDS/LOCKSWITCH.LOCKSWITCH" 1.0 1.0 0.0 null null)
                (set `self.Answer4` "4")
                (`self.Check_Answer`))
              (:`5`
                (`SkeletalMeshComponent.PlayAnimation` _r4 "/Game/untitled_category/untitled_asset/animations/RLR6.RLR6" false)
                (`GameplayStatics.PlaySound2D` "/Game/REBORN/SOUNDS/LOCKSWITCH.LOCKSWITCH" 1.0 1.0 0.0 null null)
                (set `self.Answer4` "5")
                (`self.Check_Answer`)))
            (elif (== _mainswitch 4)
              ;[1 1 1] 5
              (bind _output_get_5 (set `self.switch1` (- _switch1_4 1)))
              (if (< _switch1_4 0)
                (set `self.switch1` (+ _switch1_4 6)))
              (`KismetSystemLibrary.PrintString` (`KismetStringLibrary.Conv_IntToString` _output_get_5))
              (switch `int` (`self.switch1`) :!label _label_6
                (:`0`
                  (`SkeletalMeshComponent.PlayAnimation` _r5 "/Game/untitled_category/untitled_asset/animations/RLR1.RLR1" false)
                  (`GameplayStatics.PlaySound2D` "/Game/REBORN/SOUNDS/LOCKSWITCH.LOCKSWITCH" 1.0 1.0 0.0 null null)
                  (set `self.Answer5` "0")
                  (`self.Check_Answer`))
                (:`1`
                  (`SkeletalMeshComponent.PlayAnimation` _r5 "/Game/untitled_category/untitled_asset/animations/RLR2.RLR2" false)
                  (`GameplayStatics.PlaySound2D` "/Game/REBORN/SOUNDS/LOCKSWITCH.LOCKSWITCH" 1.0 1.0 0.0 null null)
                  (set `self.Answer5` "1")
                  (`self.Check_Answer`))
                (:`2`
                  (`SkeletalMeshComponent.PlayAnimation` _r5 "/Game/untitled_category/untitled_asset/animations/RLR3.RLR3" false)
                  (`GameplayStatics.PlaySound2D` "/Game/REBORN/SOUNDS/LOCKSWITCH.LOCKSWITCH" 1.0 1.0 0.0 null null)
                  (set `self.Answer5` "2")
                  (`self.Check_Answer`))
                (:`3`
                  (`SkeletalMeshComponent.PlayAnimation` _r5 "/Game/untitled_category/untitled_asset/animations/RLR4.RLR4" false)
                  (`GameplayStatics.PlaySound2D` "/Game/REBORN/SOUNDS/LOCKSWITCH.LOCKSWITCH" 1.0 1.0 0.0 null null)
                  (set `self.Answer5` "3")
                  (`self.Check_Answer`))
                (:`4`
                  (`SkeletalMeshComponent.PlayAnimation` _r5 "/Game/untitled_category/untitled_asset/animations/RLR5.RLR5" false)
                  (`GameplayStatics.PlaySound2D` "/Game/REBORN/SOUNDS/LOCKSWITCH.LOCKSWITCH" 1.0 1.0 0.0 null null)
                  (set `self.Answer5` "4")
                  (`self.Check_Answer`))
                (:`5`
                  (`SkeletalMeshComponent.PlayAnimation` _r5 "/Game/untitled_category/untitled_asset/animations/RLR6.RLR6" false)
                  (`GameplayStatics.PlaySound2D` "/Game/REBORN/SOUNDS/LOCKSWITCH.LOCKSWITCH" 1.0 1.0 0.0 null null)
                  (set `self.Answer5` "5")
                  (`self.Check_Answer`)))
              (elif (== _mainswitch 5)
                ;[1 1 1] 6
                (bind _output_get_6 (set `self.switch1` (- _switch1_2 1)))
                (if (< _switch1_2 0)
                  (set `self.switch1` (+ _switch1_2 6)))
                (`KismetSystemLibrary.PrintString` (`KismetStringLibrary.Conv_IntToString` _output_get_6))
                (switch `int` (`self.switch1`) :!label _label_7
                  (:`0`
                    (`SkeletalMeshComponent.PlayAnimation` _r6 "/Game/untitled_category/untitled_asset/animations/RLR1.RLR1" false)
                    (`GameplayStatics.PlaySound2D` "/Game/REBORN/SOUNDS/LOCKSWITCH.LOCKSWITCH" 1.0 1.0 0.0 null null)
                    (set `self.Naswer6` "0")
                    (`self.Check_Answer`))
                  (:`1`
                    (`SkeletalMeshComponent.PlayAnimation` _r6 "/Game/untitled_category/untitled_asset/animations/RLR2.RLR2" false)
                    (`GameplayStatics.PlaySound2D` "/Game/REBORN/SOUNDS/LOCKSWITCH.LOCKSWITCH" 1.0 1.0 0.0 null null)
                    (set `self.Naswer6` "1")
                    (`self.Check_Answer`))
                  (:`2`
                    (`SkeletalMeshComponent.PlayAnimation` _r6 "/Game/untitled_category/untitled_asset/animations/RLR3.RLR3" false)
                    (`GameplayStatics.PlaySound2D` "/Game/REBORN/SOUNDS/LOCKSWITCH.LOCKSWITCH" 1.0 1.0 0.0 null null)
                    (set `self.Naswer6` "2")
                    (`self.Check_Answer`))
                  (:`3`
                    (`SkeletalMeshComponent.PlayAnimation` _r6 "/Game/untitled_category/untitled_asset/animations/RLR4.RLR4" false)
                    (`GameplayStatics.PlaySound2D` "/Game/REBORN/SOUNDS/LOCKSWITCH.LOCKSWITCH" 1.0 1.0 0.0 null null)
                    (set `self.Naswer6` "3")
                    (`self.Check_Answer`))
                  (:`4`
                    (`SkeletalMeshComponent.PlayAnimation` _r6 "/Game/untitled_category/untitled_asset/animations/RLR5.RLR5" false)
                    (`GameplayStatics.PlaySound2D` "/Game/REBORN/SOUNDS/LOCKSWITCH.LOCKSWITCH" 1.0 1.0 0.0 null null)
                    (set `self.Naswer6` "4")
                    (`self.Check_Answer`))
                  (:`5`
                    (`SkeletalMeshComponent.PlayAnimation` _r6 "/Game/untitled_category/untitled_asset/animations/RLR6.RLR6" false)
                    (`GameplayStatics.PlaySound2D` "/Game/REBORN/SOUNDS/LOCKSWITCH.LOCKSWITCH" 1.0 1.0 0.0 null null)
                    (set `self.Naswer6` "5")
                    (`self.Check_Answer`)))))))))))

(event `Key|MouseScrollDown`
  (params (Key :type "Key Structure"))
  (bind _switch1 (`self.switch1`))
  (bind _switch1_2 (`self.switch1`))
  (bind _switch1_3 (`self.switch1`))
  (bind _switch1_4 (`self.switch1`))
  (bind _switch1_5 (`self.switch1`))
  (bind _switch1_6 (`self.switch1`))
  (bind _mainswitch (`self.MainSwitch`))
  (:`Pressed`
    (if (== _mainswitch 0)
      ;[1 1 1] 1
      (bind _output_get (set `self.switch1` (+ _switch1 1)))
      (if (> _switch1 5)
        (set `self.switch1` 0))
      (`KismetSystemLibrary.PrintString` (`KismetStringLibrary.Conv_IntToString` _output_get))
      (goto _label_2)
      (elif (== _mainswitch 1)
        ;[1 1 1] 2
        (bind _output_get_2 (set `self.switch1` (+ _switch1_3 1)))
        (if (> _switch1_3 5)
          (set `self.switch1` 0))
        (`KismetSystemLibrary.PrintString` (`KismetStringLibrary.Conv_IntToString` _output_get_2))
        (goto _label_3)
        (elif (== _mainswitch 2)
          ;[1 1 1] 3
          (bind _output_get_3 (set `self.switch1` (+ _switch1_5 1)))
          (if (> _switch1_5 5)
            (set `self.switch1` 0))
          (`KismetSystemLibrary.PrintString` (`KismetStringLibrary.Conv_IntToString` _output_get_3))
          (goto _label_4)
          (elif (== _mainswitch 3)
            ;[1 1 1] 4
            (bind _output_get_4 (set `self.switch1` (+ _switch1_6 1)))
            (if (> _switch1_6 5)
              (set `self.switch1` 0))
            (`KismetSystemLibrary.PrintString` (`KismetStringLibrary.Conv_IntToString` _output_get_4))
            (goto _label_5)
            (elif (== _mainswitch 4)
              ;[1 1 1] 5
              (bind _output_get_5 (set `self.switch1` (+ _switch1_4 1)))
              (if (> _switch1_4 5)
                (set `self.switch1` 0))
              (`KismetSystemLibrary.PrintString` (`KismetStringLibrary.Conv_IntToString` _output_get_5))
              (goto _label_6)
              (elif (== _mainswitch 5)
                ;[1 1 1] 6
                (bind _output_get_6 (set `self.switch1` (+ _switch1_2 1)))
                (if (> _switch1_2 5)
                  (set `self.switch1` 0))
                (`KismetSystemLibrary.PrintString` (`KismetStringLibrary.Conv_IntToString` _output_get_6))
                (goto _label_7)))))))))

(fn `UserConstructionScript`)