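; Keypad door lock that takes a typed code on number keys, with E calling back the camera.
; Each key plays a button montage and sound, updates dynamic-material digit lights, and appends to a string in ChecandoPalavra.
; When the digit countdown ends, a match with RespostaCerta lights green, disables input and calls DestroyTrigger after a delay.
; A mismatch resets the entry and flashes the status light through a timeline with an error sound.
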(event `self.ReceiveBeginPlay`
  ;[1 1 1] tem que sair da mesh
  (bind _returnvalue (`PrimitiveComponent.CreateDynamicMaterialInstance` (`self.Alarm`) 1 "/Game/REBORN/MATERIALS/AlarmL1.AlarmL1" "None"))
  (set `self.L1` _returnvalue)
  ;[1 1 1] tem que sair do return value do create dynamic material instance
  (`MaterialInstanceDynamic.SetVectorParameterValue` (`self.L1`) "Shine" (struct :`A` 1.0))
  (bind _returnvalue_2 (`PrimitiveComponent.CreateDynamicMaterialInstance` (`self.Alarm`) 2 "/Game/REBORN/MATERIALS/AlarmL2.AlarmL2" "None"))
  (set `self.L2` _returnvalue_2)
  (`MaterialInstanceDynamic.SetVectorParameterValue` _returnvalue_2 "Shine" (struct :`A` 1.0))
  (bind _returnvalue_3 (`PrimitiveComponent.CreateDynamicMaterialInstance` (`self.Alarm`) 3 "/Game/REBORN/MATERIALS/AlarmL3.AlarmL3" "None"))
  (set `self.L3` _returnvalue_3)
  (`MaterialInstanceDynamic.SetVectorParameterValue` _returnvalue_3 "Shine" (struct :`A` 1.0))
  (bind _returnvalue_4 (`PrimitiveComponent.CreateDynamicMaterialInstance` (`self.Alarm`) 4 "/Game/REBORN/MATERIALS/AlarmL4.AlarmL4" "None"))
  (set `self.L4` _returnvalue_4)
  (`MaterialInstanceDynamic.SetVectorParameterValue` _returnvalue_4 "Shine" (struct :`A` 1.0))
  (bind _returnvalue_5 (`PrimitiveComponent.CreateDynamicMaterialInstance` (`self.Alarm`) 5 "/Game/REBORN/MATERIALS/AlarmL5.AlarmL5" "None"))
  (set `self.L5` _returnvalue_5)
  (`MaterialInstanceDynamic.SetVectorParameterValue` _returnvalue_5 "Shine" (struct :`A` 1.0))
  (bind _returnvalue_6 (`PrimitiveComponent.CreateDynamicMaterialInstance` (`self.Alarm`) 6 "/Game/REBORN/MATERIALS/AlarmL6.AlarmL6" "None"))
  (set `self.L6` _returnvalue_6)
  (bind (_direction _newtrack_0) (`Timeline|Timeline_0`)
    (:`Update`
      (`MaterialInstanceDynamic.SetVectorParameterValue` _returnvalue_6 "Shine" (`KismetMathLibrary.Conv_VectorToLinearColor` _newtrack_0))
      (`self.DisableInput` (`GameplayStatics.GetPlayerController` 0) null))))

(event `Key|One`
  (params (Key :type "Key Structure"))
  (:`Pressed`
    (set `self.Key` 0)
    (`self.Check_Click`)))

(event `Key|Two`
  (params (Key :type "Key Structure"))
  (:`Pressed`
    (set `self.Key` 1)
    (`self.Check_Click`)))

(event `Check_Click`
  (`self.Tecla` (`self.Key`)))

(event `LightAnswer`
  (switch `int` (`self.TotalDigitos`)
    (:`0`
      (`MaterialInstanceDynamic.SetVectorParameterValue` (`self.L1`) "Shine" (struct :`R` 1.0 :`G` 1.5 :`B` 1.0 :`A` 1.0) :!label _label)
      (`MaterialInstanceDynamic.SetVectorParameterValue` (`self.L2`) "Shine" (struct :`R` 1.0 :`G` 1.5 :`B` 1.0 :`A` 1.0))
      (`MaterialInstanceDynamic.SetVectorParameterValue` (`self.L3`) "Shine" (struct :`R` 1.0 :`G` 1.5 :`B` 1.0 :`A` 1.0))
      (`MaterialInstanceDynamic.SetVectorParameterValue` (`self.L4`) "Shine" (struct :`R` 1.0 :`G` 1.5 :`B` 1.0 :`A` 1.0)))
    (:`1`
      (goto _label))
    (:`2`
      (`MaterialInstanceDynamic.SetVectorParameterValue` (`self.L1`) "Shine" (struct :`R` 1.0 :`G` 1.5 :`B` 1.0 :`A` 1.0))
      (`MaterialInstanceDynamic.SetVectorParameterValue` (`self.L2`) "Shine" (struct :`R` 1.0 :`G` 1.5 :`B` 1.0 :`A` 1.0))
      (`MaterialInstanceDynamic.SetVectorParameterValue` (`self.L3`) "Shine" (struct :`R` 1.0 :`G` 1.5 :`B` 1.0 :`A` 1.0))
      (`MaterialInstanceDynamic.SetVectorParameterValue` (`self.L4`) "Shine" (struct :`A` 1.0)))
    (:`3`
      (`MaterialInstanceDynamic.SetVectorParameterValue` (`self.L1`) "Shine" (struct :`R` 1.0 :`G` 1.5 :`B` 1.0 :`A` 1.0))
      (`MaterialInstanceDynamic.SetVectorParameterValue` (`self.L2`) "Shine" (struct :`R` 1.0 :`G` 1.5 :`B` 1.0 :`A` 1.0))
      (`MaterialInstanceDynamic.SetVectorParameterValue` (`self.L3`) "Shine" (struct :`A` 1.0))
      (`MaterialInstanceDynamic.SetVectorParameterValue` (`self.L4`) "Shine" (struct :`A` 1.0)))
    (:`4`
      (`MaterialInstanceDynamic.SetVectorParameterValue` (`self.L1`) "Shine" (struct :`R` 1.0 :`G` 1.5 :`B` 1.0 :`A` 1.0))
      (`MaterialInstanceDynamic.SetVectorParameterValue` (`self.L2`) "Shine" (struct :`A` 1.0))
      (`MaterialInstanceDynamic.SetVectorParameterValue` (`self.L3`) "Shine" (struct :`A` 1.0))
      (`MaterialInstanceDynamic.SetVectorParameterValue` (`self.L4`) "Shine" (struct :`A` 1.0)))))

(event `Key|Three`
  (params (Key :type "Key Structure"))
  (:`Pressed`
    (set `self.Key` 2)
    (`self.Check_Click`)))

(event `Key|Four`
  (params (Key :type "Key Structure"))
  (:`Pressed`
    (set `self.Key` 3)
    (`self.Check_Click`)))

(event `Key|Five`
  (params (Key :type "Key Structure"))
  (:`Pressed`
    (set `self.Key` 4)
    (`self.Check_Click`)))

(event `ChecarTecla`
  (params (component :type "PrimitiveComponent Object Reference")))

(event `Key|Six`
  (params (Key :type "Key Structure"))
  (:`Pressed`
    (set `self.Key` 5)
    (`self.Check_Click`)))

(event `Key|Seven`
  (params (Key :type "Key Structure"))
  (:`Pressed`
    (set `self.Key` 6)
    (`self.Check_Click`)))

(event `Key|Eight`
  (params (Key :type "Key Structure"))
  (:`Pressed`
    (set `self.Key` 7)
    (`self.Check_Click`)))

(event `Key|Nine`
  (params (Key :type "Key Structure"))
  (:`Pressed`
    (set `self.Key` 8)
    (`self.Check_Click`)))

(event `Key|Zero`
  (params (Key :type "Key Structure"))
  (:`Pressed`
    (set `self.Key` 9)
    (`self.Check_Click`)))

(event `Key|E`
  (params (Key :type "Key Structure"))
  (:`Pressed`
    (set `self.Key` 10)
    (`self.Check_Click`)))

(event `Acertou`
  (`KismetSystemLibrary.PrintString` "Acertou Mizeravi!")
  (`MaterialInstanceDynamic.SetVectorParameterValue` (`self.L5`) "Shine" (struct :`R` 0.001685 :`G` 1.0 :`A` 1.0))
  (`self.DisableInput` (`GameplayStatics.GetPlayerController` 0))
  (`GameplayStatics.PlaySound2D` "/Game/REBORN/SOUNDS/CORRECT.CORRECT" 1.0 1.0 0.0 null null)
  (`KismetSystemLibrary.Delay` 0.4)
  (`self.CorrectAnswer`))

(event `CorrectAnswer`
  (`self.DestroyTrigger`))

(event `RetornoCamera`
  (`self.BackCAMERA`))

(event `Errou`
  (`KismetSystemLibrary.PrintString` "Errooouu!")
  (`GameplayStatics.PlaySound2D` "/Game/REBORN/SOUNDS/WRONG.WRONG" 1.0 1.0 0.0 null null)
  (bind (_direction _newtrack_0) (`Timeline|Timeline_1` :!via `PlayFromStart`)
    (:`Update`
      (`MaterialInstanceDynamic.SetVectorParameterValue` (`self.L5`) "Shine" (`KismetMathLibrary.Conv_VectorToLinearColor` _newtrack_0))
      (`KismetSystemLibrary.RetriggerableDelay` 0.2)
      (`MaterialInstanceDynamic.SetVectorParameterValue` (`self.L5`) "Shine" (struct :`A` 1.0)))))

(event `ResetarTexto`
  ;[1 1 1] Reset
  (set `self.TotalDigitos` 4)
  (set `self.textoDigitado` "")
  (`MaterialInstanceDynamic.SetVectorParameterValue` (`self.L1`) "Shine" (struct :`A` 1.0))
  (`MaterialInstanceDynamic.SetVectorParameterValue` (`self.L2`) "Shine" (struct :`A` 1.0))
  (`MaterialInstanceDynamic.SetVectorParameterValue` (`self.L3`) "Shine" (struct :`A` 1.0))
  (`MaterialInstanceDynamic.SetVectorParameterValue` (`self.L4`) "Shine" (struct :`A` 1.0))
  (`MaterialInstanceDynamic.SetVectorParameterValue` (`self.L5`) "Shine" (struct :`A` 1.0)))

(fn `UserConstructionScript`)